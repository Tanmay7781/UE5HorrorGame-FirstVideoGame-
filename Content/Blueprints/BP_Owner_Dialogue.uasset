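; One-shot trigger actor that shows the owner's dialogue when the first-person player walks into it.
; On player overlap it destroys its trigger box and applies a fixed local rotation to the actor in BPFPref.
; It then adds a BP_OwnerDialogue widget to the viewport and removes it after a timed delay.
; Nodes for disabling and re-enabling player input are present but unconnected.
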(event OnComponentBeginOverlap(TriggerBox)
  (params (OverlappedComponent :type Primitive%20Component%20Object%20Reference) (OtherActor :type Actor%20Object%20Reference) (OtherComp :type Primitive%20Component%20Object%20Reference) (OtherBodyIndex :type Integer) (bFromSweep :type Boolean) (SweepResult :type Hit%20Result%20Structure%20%28by%20ref%29))
  (Utilities|Casting|CastToBP_FirstPersonCharacter OtherActor)
  (Variables|Default|SetIsPlayerNearby true)
  (Components|DestroyComponent (Variables|Default|GetTriggerBox))
  (if (Variables|Default|GetIsPlayerNearby)
    (Transformation|AddActorLocalRotation (Variables|Default|GetBP_FPref) "0.000000,40.000000,0.000000" false false)
    (bind _returnvalue (UserInterface|CreateWidget "/Game/Blueprints/BP_OwnerDialogue.BP_OwnerDialogue_C"))
    (UserInterface|Viewport|AddtoViewport _returnvalue 0)
    (Utilities|FlowControl|Delay 12.0)
    (Widget|RemovefromParent _returnvalue)))

(event EventBeginPlay)

(event Collision|EventActorBeginOverlap
  (params (OtherActor :type Actor%20Object%20Reference)))

(event EventTick
  (params (DeltaSeconds :type Float%20%28single-precision%29)))

(fn ConstructionScript)
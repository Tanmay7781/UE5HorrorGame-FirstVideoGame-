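; Trigger actor that stages a one-time scripted power outage when the first-person character enters a room.
; Overlap destroys the trigger box, freezes the referenced closet's physics and, after a delay, disables player input while a timeline dims the assigned lights.
; A DoOnce inside the per-light update shows a temporary outage widget, then reverses the timeline and restores physics and input.
; Event dispatchers signal lights off, lights on and widget removal.
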(event Collision|EventActorBeginOverlap
  (params (OtherActor :type Actor%20Object%20Reference))
  (Utilities|Casting|CastToBP_FirstPersonCharacter OtherActor)
  (bind _output_get (Variables|Default|SetIsPlayerinRoom true))
  (Components|DestroyComponent (Variables|Default|GetTriggerbox))
  (Physics|SetSimulatePhysics (Variables|/Game/Blueprints/BP_Closet.BP_Closet_C|Getantique_closet_mid_poly (Variables|Default|GetCbrd%20Ref)) false)
  (if _output_get
    (Utilities|FlowControl|Delay 2.0)
    (Input|DisableInput (Game|GetPlayerCharacter 0) (Game|GetPlayerController 0))
    (bind _powerdown (Timeline|PowerOutage Play)
      (:Update
        (for _array_element (Variables|Default|GetLights)
          (Rendering|Components|Light|SetIntensity (Variables|/Script/Engine.Light|GetLightComponent _array_element) _powerdown)
          (Variables|Default|SetLightsoff true)
          (Default|CallOnlightsoff)
          (Utilities|FlowControl|Delay 5.0)
          (Utilities|FlowControl|DoOnce false
            (:Completed
              (bind _returnvalue (UserInterface|CreateWidget "/Game/Blueprints/BP_POWidget.BP_POWidget_C"))
              (bind _output_get_2 (Variables|Default|SetPOUIWidg _returnvalue))
              (UserInterface|Viewport|AddtoViewport _output_get_2 0)
              (Utilities|FlowControl|Delay 1e+01)
              (Widget|RemovefromParent _output_get_2)
              (Utilities|FlowControl|Sequence
                (:then_0
                  (if (Variables|Default|GetLightsoff)
                    (Utilities|FlowControl|Delay 5.0)
                    (Variables|Default|SetLightsoff false)
                    (Default|CallOnlightson)
                    (Physics|SetSimulatePhysics (Variables|/Game/Blueprints/BP_Closet.BP_Closet_C|Getantique_closet_mid_poly (Variables|Default|GetCbrd%20Ref)) true)
                    (Input|EnableInput (Game|GetPlayerCharacter 0) (Game|GetPlayerController 0))
                    (Timeline|PowerOutage Reverse)))
                (:then_1
                  (Utilities|FlowControl|Delay 4.0)
                  (Default|CallOnWidgetDestroyed))))))))))

(fn ConstructionScript)
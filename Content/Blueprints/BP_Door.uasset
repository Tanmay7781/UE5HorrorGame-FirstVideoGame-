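; BP_Door is an interactive swinging door that the first-person player toggles with E while inside its TriggerBox.
; Tick polls the key and, after a short Delay, plays or reverses a timeline rotating DoorPivot, with a door sound.
; At BeginPlay it binds to BP_PowerOutage's lights-off event, which auto-closes an open door once, after a delay.
; AvoidCollision toggle events exist, but their power-outage bindings never run.
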(event OnComponentEndOverlap(TriggerBox)
  (params (OverlappedComponent :type Primitive%20Component%20Object%20Reference) (OtherActor :type Actor%20Object%20Reference) (OtherComp :type Primitive%20Component%20Object%20Reference) (OtherBodyIndex :type Integer))
  (Utilities|Casting|CastToBP_FirstPersonCharacter OtherActor)
  (Variables|Default|SetbIsPlayerNearby false))

(event OnComponentBeginOverlap(TriggerBox)
  (params (OverlappedComponent :type Primitive%20Component%20Object%20Reference) (OtherActor :type Actor%20Object%20Reference) (OtherComp :type Primitive%20Component%20Object%20Reference) (OtherBodyIndex :type Integer) (bFromSweep :type Boolean) (SweepResult :type Hit%20Result%20Structure%20%28by%20ref%29))
  (Utilities|Casting|CastToBP_FirstPersonCharacter OtherActor)
  (Variables|Default|SetbIsPlayerNearby true))

(event Custom|AutoCloseDoors
  (Utilities|FlowControl|DoOnce false
    (:Completed
      (Utilities|FlowControl|Delay 3.0)
      (if (Variables|Default|GetIsDoorOpen)
        (Variables|Default|SetIsDoorOpen false)
        (bind _dooropen (Timeline|OpenDoorTimeline Reverse)
          (:Update
            (Transformation|SetRelativeRotation (Variables|Default|GetDoorPivot) (Math|Rotator|MakeRotator 0.0 0.0 _dooropen) false false)))))))

(event Custom|DoorAllowed
  (Collision|SetCollisionEnabled (Variables|Default|GetAvoidCollision) "QueryAndPhysics"))

(event Custom|DoorNotAllowed
  (Collision|SetCollisionEnabled (Variables|Default|GetAvoidCollision) "NoCollision"))

(event EventBeginPlay
  (Utilities|FlowControl|DoOnce false
    (:Completed
      (bind _outactors (Actor|GetAllActorsOfClass "/Game/Blueprints/BP_PowerOutage.BP_PowerOutage_C"))
      (EventDispatchers|BindEventtoOnlightsoff _outactors (delegate Custom|AutoCloseDoors)))))

(event Collision|EventActorBeginOverlap
  (params (OtherActor :type Actor%20Object%20Reference)))

(event EventTick
  (params (DeltaSeconds :type Float%20%28single-precision%29))
  (bind _returnvalue (Game|GetPlayerController 0))
  (bind _returnvalue_2 (Game|Player|IsInputKeyDown _returnvalue "E"))
  (if (Variables|Default|GetbIsPlayerNearby)
    (if (Variables|Default|GetIsDoorOpen)
      (if _returnvalue_2
        (Utilities|FlowControl|Delay 0.5)
        (Variables|Default|SetIsDoorOpen false)
        (Audio|PlaySound2D "/Game/ImportedAudio/door.door" 1.0 1.0 0.0 0 0)
        (bind _dooropen (Timeline|OpenDoorTimeline Reverse)
          (:Update
            (Transformation|SetRelativeRotation (Variables|Default|GetDoorPivot) (Math|Rotator|MakeRotator 0.0 0.0 _dooropen) false false))))
      (elif _returnvalue_2
        (Utilities|FlowControl|Delay 0.5)
        (Variables|Default|SetIsDoorOpen true)
        (Audio|PlaySound2D "/Game/ImportedAudio/door.door" 1.0 1.0 0.0 0 0)
        (Timeline|OpenDoorTimeline Play)))))

(fn ConstructionScript)